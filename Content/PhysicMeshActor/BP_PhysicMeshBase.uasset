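; Base actor for connectable mesh pieces that attach to one another through ConnectPointComponents, exposed via interface functions.
; It gives each piece a random color and a random ID tag, and swaps to M_Tran while hit.
; Connection queries gather points across the whole attachment hierarchy from the top actor.
; Breaking detaches it from parent and children and resets their tags, caching the child list so detaching doesn't break the loop.
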(event EventBPIToggleHitState
  (params (bHit :type Boolean))
  (bind _staticmesh (Variables|Default|GetStaticMesh))
  (if bHit
    (Rendering|Material|SetMaterial _staticmesh 0 "/PhysicAssemblySystem/Material/M_Tran.M_Tran")
    (else
      (Rendering|Material|SetMaterial _staticmesh 0 (Variables|Default|GetMID)))))

(event EventBeginPlay
  ;[1 0.04688 0] begin
  (Utilities|FlowControl|Sequence
    (:then_0
      (Variables|Default|SetConnectPointList (Actor|GetComponentsByClass "/Script/PhysicAssemblySystem.ConnectPointComponent")))
    (:then_1
      ;[0 0.8828 1] random id to mask unique object
      (Variables|Default|SetID (Math|Random|RandomInteger 2147483647))
      (Utilities|Array|AddUnique (Variables|Actor|GetTags) (Utilities|String|StringToName (Utilities|String|ToString(Integer) (Variables|Default|GetID)))))))

(event EventBPIBreakConnect
  ;[0 1 0.01562] break
  (Utilities|FlowControl|Sequence
    (:then_0
      ;[1 0.3281 0] has parent , detach from parent + reset tag
      (Utilities|IsValid (Actor|GetAttachParentActor)
        (:Is%20Valid
          (Transformation|DetachFromActor "KeepWorld" "KeepWorld" "KeepWorld")
          ;[0.07812 0 1] reset self tag
          (CallFunction|BPIResetTag))))
    (:then_1
      ;[1 0 0.1875] detach all directly child
      (bind _output_get (Variables|Default|SetCacheTempChildActors (Actor|GetAttachedActors true))) ; add var to protect detach break loop
      (for _array_element _output_get
        ;;[0 1 0.2031] detach will break loop
        (Transformation|DetachFromActor _array_element "KeepWorld" "KeepWorld" "KeepWorld")
        (Class|BPIMesh|BPIResetTag(Message) _array_element)))))

(event EventBPIResetTag
  ;[0.4062 0 1] reset tag
  (Class|LibPhysicSystemHelper|LibResetTag self (Variables|Default|GetID)))

(fn ConstructionScript
  (bind _returnvalue (Rendering|Material|CreateDynamicMaterialInstance (Variables|Default|GetStaticMesh) 0 "/PhysicAssemblySystem/Material/MI_Mesh.MI_Mesh" "None" :!class /Script/Engine.PrimitiveComponent))
  (Variables|Default|SetMID _returnvalue)
  (bind _output_get (Variables|Default|SetInitColor (Class|LibHelper|LibMakeRandomLinearColor)))
  (Rendering|Material|SetVectorParameterValue (Variables|Default|GetMID) "color" _output_get :!class /Script/Engine.MaterialInstanceDynamic))

(fn BPIGetAllConnectPointList
  (for _array_element (Class|LibPhysicSystemHelper|LibGetAllChildActor (Class|LibPhysicSystemHelper|LibFindTopActor self))
    (bind _connectpoints (Class|BPIMesh|BPIGetConnectPointList(Message) _array_element))
    (Class|LibPhysicSystemHelper|LibAppendto (LocalVariables|GetTmpList) _connectpoints))
  (return (LocalVariables|GetTmpList)))

(fn BPIGetConnectPointList
  (return (Variables|Default|GetConnectPointList)))

(fn BPIGetPrimitiveComponent
  (return (Variables|Default|GetStaticMesh)))

(fn BPIGetUniqueID
  (return (Variables|Default|GetID)))