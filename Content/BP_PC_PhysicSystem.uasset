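; Player controller for a physics-based mesh assembly system where the player grabs, snaps, connects and detaches parts.
; Assembly mode (Z) highlights the aimed actor, which left mouse grabs with a PhysicsHandle at wheel-adjusted distance.
; While moving, a sphere trace finds the best connection-point pair, drawn with debug shapes, for V snapping and F attachment with tag updates.
; Right mouse breaks connections, and releasing a grab eases velocity to zero through a timeline.
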(event EventBeginPlay
  ;[0 1 0.2734] beign
  (Utilities|FlowControl|Sequence
    (:then_0
      (bind _returnvalue (UserInterface|CreateWidget "/PhysicAssemblySystem/UI/UI_HUD.UI_HUD_C" self))
      (UserInterface|Viewport|AddtoViewport _returnvalue 0))
    (:then_1
      (bind _returnvalue_2 (UserInterface|CreateWidget "/PhysicAssemblySystem/UI/UI_DebugInfo.UI_DebugInfo_C" self))
      (bind _output_get (Variables|Default|SetUI_DebugInfo _returnvalue_2))
      (UserInterface|Viewport|AddtoViewport _output_get 0))))

(event EventTick
  (params (DeltaSeconds :type Float%20%28single-precision%29))
  (bind (_start _end) (CallFunction|GetStartandEnd 999999.0))
  ;[0.9922 0 1] tick
  (Utilities|FlowControl|Sequence
    (:then_0
      (switch Utilities|FlowControl|Switch|SwitchonEPhysicMode (Variables|Default|GetCurrentMode)
        (:NewEnumerator0
          (bind (_outhit _returnvalue) (Collision|LineTraceByChannel _start _end "TraceTypeQuery1" false 0 "None"))
          (if _returnvalue
            (Utilities|FlowControl|Sequence
              (:then_0
                ;[0.6641 0 1] cancel old mesh's active
                (bind _hitactor (Variables|Default|GetHitActor :!label _label)
                  (:then
                    (Class|BPIMesh|BPIToggleHitState(Message) _hitactor false))
                  (:else)))
              (:then_1
                (bind _output_get (Variables|Default|SetHitActor (.HitActor (Collision|BreakHitResult _outhit))))
                (Class|BPIMesh|BPIToggleHitState(Message) _output_get true)
                (Variables|Default|SetImpactPoint (.ImpactPoint (Collision|BreakHitResult _outhit)))))
            (else
              (goto _label))))
        (:NewEnumerator2
          (Utilities|FlowControl|Sequence
            (:then_0
              (|FindBestPathAndCacheHitResult))
            (:then_1
              (|CalcHandTargetPosAndHandleAdsorb))
            (:then_2
              (|DrawHitResultInfo))
            (:then_3
              (|DrawBestPathLine))))))
    (:then_1
      (CallFunction|ShowDebugInfo))))

(event Input|MouseEvents|MouseWheelAxis
  (params (AxisValue :type Float%20%28single-precision%29))
  ;[0 1 0.4609] update radius
  (Variables|Default|SetLength (+ (Variables|Default|GetLength) (* AxisValue 5e+01))))

(event Input|KeyboardEvents|Z
  (params (Key :type Key%20Structure :default "None"))
  ;[1 0.9141 0] z key join assembly mode
  (:Pressed
    (Variables|Default|SetLastMode (Variables|Default|GetCurrentMode))
    (Variables|Default|SetCurrentMode "NewEnumerator0")))

(event Input|MouseEvents|LeftMouseButton
  (params (Key :type Key%20Structure :default "None"))
  ;[0 1 0.5313] left mouse button
  (:Pressed
    (Variables|Default|SetLastMode (Variables|Default|GetCurrentMode))
    (Variables|Default|SetCurrentMode "NewEnumerator2")
    (bind _hitactor (Variables|Default|GetHitActor)
      (:then
        (bind _component (Class|BPIMesh|BPIGetPrimitiveComponent(Message) _hitactor))
        (Physics|Components|PhysicsHandle|GrabComponentatLocationwithRotation (Variables|Default|GetPhysicsHandle) _component "None" (Variables|Default|GetImpactPoint) "0, 0, 0"))
      (:else)))
  (:Released
    (Utilities|FlowControl|Sequence
      (:then_0
        (Physics|Components|PhysicsHandle|ReleaseComponent (Variables|Default|GetPhysicsHandle))
        (bind _hitactor_2 (Variables|Default|GetHitActor)
          (:then
            (bind _component_2 (Class|BPIMesh|BPIGetPrimitiveComponent(Message) _hitactor_2))
            (Utilities|IsValid _component_2
              (:Is%20Valid
                (bind _returnvalue (Physics|GetPhysicsLinearVelocity _component_2 "None"))
                (Variables|Default|SetSpeedStart _returnvalue)
                (Components|Timeline|SetPlayRate (Variables|Default|GetTL) (/ 1.0 0.5))
                (bind _0_1 (Timeline|TL PlayFromStart)
                  (:Update
                    (Physics|SetPhysicsLinearVelocity _component_2 (Math|Vector|Lerp(Vector) (Variables|Default|GetSpeedStart) "0, 0, 0" _0_1) false "None"))))))
          (:else)))
      (:then_1
        (Variables|Default|SetCurrentMode (Variables|Default|GetLastMode))
        (Variables|Default|SetRoll 0.0)
        (Variables|Default|SetPitch 0.0)
        (Variables|Default|SetYaw 0.0)))))

(event Input|KeyboardEvents|F
  (params (Key :type Key%20Structure :default "None"))
  (bind _bestpath (Variables|Default|GetBestPath))
  (bind (_tracedcomponent _selfcomponent) (Utilities|Struct|BreakConnectPath _bestpath))
  (bind _returnvalue (Components|GetOwner _tracedcomponent))
  (bind _returnvalue_2 (Components|GetOwner _selfcomponent))
  ;[0.6406 0 1] F key to Assembly mesh
  (:Pressed
    (switch Utilities|FlowControl|Switch|SwitchonEPhysicMode (Variables|Default|GetCurrentMode)
      (:NewEnumerator2
        (if (Variables|Default|GetbHasBestPath)
          (Transformation|AttachActorToActor _returnvalue_2 _returnvalue "None" "KeepWorld" "KeepWorld" "KeepWorld" true)
          ;[0.2422 1 0] update tag
          (Class|LibPhysicSystemHelper|LibUpdateTagwhenConnect _returnvalue _returnvalue_2))))))

(event Input|MouseEvents|RightMouseButton
  (params (Key :type Key%20Structure :default "None"))
  (bind (_start _end) (CallFunction|GetStartandEnd 9999999.0))
  ;[1 0.1406 0] right mouse button to break connect
  (:Pressed
    (bind (_outhit _returnvalue) (Collision|LineTraceByChannel _start _end "TraceTypeQuery1" true 0 "None"))
    (if _returnvalue
      (Class|BPIMesh|BPIBreakConnect(Message) (.HitActor (Collision|BreakHitResult _outhit))))))

(event Input|KeyboardEvents|V
  (params (Key :type Key%20Structure :default "None"))
  ;[0.3359 0 1] v key to toggle adsorb
  (:Pressed
    (Variables|Default|SetbAdsorb true))
  (:Released
    (Variables|Default|SetbAdsorb false)))

(fn ConstructionScript)

(fn BPGetStartandEnd
  (params (Radius :type Float%20%28single-precision%29))
  (bind _returnvalue (Pawn|GetControlledPawn))
  (bind _returnvalue_2 (Transformation|GetActorLocation _returnvalue))
  (return _returnvalue_2 (+ _returnvalue_2 (* (Math|Vector|GetForwardVector (Pawn|GetControlRotation :!class /Script/Engine.Controller)) Radius))))

(fn BPShowDebugInfo
  (bind (_start _end) (CallFunction|GetStartandEnd 999999.0))
  (bind (_outhit _returnvalue) (Collision|LineTraceByChannel _start _end "TraceTypeQuery1" false 0 "None"))
  (if _returnvalue
    (bind _asbp_physic_mesh_base (Utilities|Casting|CastToBP_PhysicMeshBase (.HitActor (Collision|BreakHitResult _outhit))))
    (bind _ui_debuginfo (Variables|Default|GetUI_DebugInfo)
      (:then
        (Default|UpdateInfo _ui_debuginfo _asbp_physic_mesh_base)
        (return))
      (:else))))

(fn BPHandleAdsorb
  (params (Pos :type Vector))
  (bind _bestpath (Variables|Default|GetBestPath))
  (bind (_tracedcomponent _selfcomponent) (Utilities|Struct|BreakConnectPath _bestpath))
  (if (Variables|Default|GetbAdsorb)
    (return (+ (- (Transformation|GetWorldLocation _tracedcomponent) (Transformation|GetWorldLocation _selfcomponent)) Pos))
    (else
      (return Pos))))